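; Checkpoint actor that records a respawn-style transform on the player kart when the kart overlaps it.
; On begin overlap it casts to BP_KartPawnPlayer and sets its CheckpointTransform from the ReferenceArrow's world location and rotation, with unit scale.
; The arrow, rather than the kart's pose, defines the saved position and facing.
; An older variant that saved and printed the kart's own transform remains disconnected.
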(event Collision|EventActorBeginOverlap
  (params (OtherActor :type Actor%20Object%20Reference))
  (bind _referencearrow (Variables|Default|GetReferenceArrow))
  (bind _returnvalue (Transformation|GetWorldTransform _referencearrow))
  ;[1 1 1] Teleport test
  (bind _asbp_kart_pawn_player (Utilities|Casting|CastToBP_KartPawnPlayer OtherActor))
  (Variables|/Game/Blueprints/VehicleBlueprints/BP_KartPawnPlayer.BP_KartPawnPlayer_C|SetCheckpoint%20Transform _asbp_kart_pawn_player (Math|Transform|MakeTransform (.location _returnvalue) (.rotation _returnvalue) "1,1,1")))

(fn ConstructionScript)
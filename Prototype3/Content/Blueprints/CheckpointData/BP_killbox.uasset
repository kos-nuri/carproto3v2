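; Kill volume actor that sends the player kart back to its last checkpoint.
; On overlap with a BP_KartPawnPlayer, it teleports player pawn 0 to the location and rotation of that kart's stored CheckpointTransform.
; An unconnected alternative that respawns, destroys and repossesses the kart is left in the graph and never runs.
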(event EventBeginPlay)

(event Collision|EventActorBeginOverlap
  (params (OtherActor :type Actor%20Object%20Reference))
  ;[1 1 1] Teleport Test
  (bind _asbp_kart_pawn_player (Utilities|Casting|CastToBP_KartPawnPlayer OtherActor))
  (Transformation|Teleport (Game|Player|GetPlayerPawn 0) (.location (Variables|/Game/Blueprints/VehicleBlueprints/BP_KartPawnPlayer.BP_KartPawnPlayer_C|GetCheckpoint%20Transform _asbp_kart_pawn_player)) (.rotation (Variables|/Game/Blueprints/VehicleBlueprints/BP_KartPawnPlayer.BP_KartPawnPlayer_C|GetCheckpoint%20Transform _asbp_kart_pawn_player))))

(event EventTick
  (params (DeltaSeconds :type Float%20%28single-precision%29)))

(fn ConstructionScript)
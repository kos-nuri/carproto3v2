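; Invisible boundary wall that slows a kart straying off the path and respawns it at its stored checkpoint.
; Overlap shows a warning widget and sets a slow flag; leaving the box clears both.
; Tick steps the kart's Acceleration down while slowed, or back up otherwise, within clamped limits.
; If acceleration is zero after a delay, it spawns a replacement kart, destroys the old one and has player 0 possess the new one.
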(event OnComponentEndOverlap(Box)
  (params (OverlappedComponent :type Primitive%20Component%20Object%20Reference) (OtherActor :type Actor%20Object%20Reference) (OtherComp :type Primitive%20Component%20Object%20Reference) (OtherBodyIndex :type Integer))
  ;[1 1 1] Sets If player returns to path
  (Variables|Default|SetIsSlowed false)
  (Widget|RemovefromParent (stale Collision|EventActorBeginOverlap _returnvalue)))

(event EventBeginPlay)

(event Collision|EventActorBeginOverlap
  (params (OtherActor :type Actor%20Object%20Reference))
  ;[1 1 1] Player Warning HUD
  (Variables|Default|SetIsSlowed true)
  (bind _returnvalue (UserInterface|CreateWidget "/Game/Blueprints/HUD/HUD_InvisibleWallWarning.HUD_InvisibleWallWarning_C"))
  (UserInterface|Viewport|AddtoViewport _returnvalue 0))

(event EventTick
  (params (DeltaSeconds :type Float%20%28single-precision%29))
  (if (Variables|Default|GetIsSlowed)
    ;[1 1 1] slows down character
    (bind _asbp_kart_pawn_player (Utilities|Casting|CastToBP_KartPawnPlayer (stale Collision|EventActorBeginOverlap OtherActor)))
    (Variables|/Game/Blueprints/VehicleBlueprints/BP_KartPawnBase.BP_KartPawnBase_C|SetAcceleration _asbp_kart_pawn_player (Math|Float|Clamp(Float) (- (Variables|/Game/Blueprints/VehicleBlueprints/BP_KartPawnBase.BP_KartPawnBase_C|GetAcceleration _asbp_kart_pawn_player) 1e+02) 0.0 4e+03))
    (Utilities|FlowControl|Delay 3.0)
    (if (<= (Variables|/Game/Blueprints/VehicleBlueprints/BP_KartPawnBase.BP_KartPawnBase_C|GetAcceleration _asbp_kart_pawn_player) 0.0)
      ;[1 1 1] spawns a dummy actor to catch player before destroying previous one
      (bind _returnvalue (Game|SpawnActorfromClass "/Game/Blueprints/VehicleBlueprints/BP_KartPawnPlayer.BP_KartPawnPlayer_C" (Variables|/Game/Blueprints/VehicleBlueprints/BP_KartPawnPlayer.BP_KartPawnPlayer_C|GetCheckpoint%20Transform _asbp_kart_pawn_player) "Undefined" 0 0))
      (Actor|DestroyActor _asbp_kart_pawn_player)
      (Pawn|Possess (Game|GetPlayerController 0) _returnvalue))
    (else
      ;[1 1 1] restores acceleration
      (bind _asbp_kart_pawn_player_2 (Utilities|Casting|CastToBP_KartPawnPlayer (stale Collision|EventActorBeginOverlap OtherActor)))
      (Variables|/Game/Blueprints/VehicleBlueprints/BP_KartPawnBase.BP_KartPawnBase_C|SetAcceleration _asbp_kart_pawn_player_2 (Math|Float|Clamp(Float) (+ (Variables|/Game/Blueprints/VehicleBlueprints/BP_KartPawnBase.BP_KartPawnBase_C|GetAcceleration _asbp_kart_pawn_player_2) 1e+02) 0.0 4e+03)))))

(fn ConstructionScript)
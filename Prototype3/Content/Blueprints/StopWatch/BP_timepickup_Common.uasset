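; BP_timepickup_Common is a time pickup that extends the game's countdown when the player's kart overlaps it.
; On overlap with BP_KartPawnPlayer, it adds five seconds to CountdownTimer in BP_GameMode.
; A DoOnce placed after that addition then decrements the game mode's CommonAmount, destroys the pickup and plays a 2D pickup sound.
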(event Collision|EventActorBeginOverlap
  (params (OtherActor :type Actor%20Object%20Reference))
  ;[1 1 1] Adds Time in BP Gamemode
  (Utilities|Casting|CastToBP_KartPawnPlayer OtherActor)
  (bind _asbp_game_mode (Utilities|Casting|CastToBP_GameMode (Game|GetGameMode)))
  (Variables|/Game/Blueprints/VehicleBlueprints/BP_GameMode.BP_GameMode_C|SetCountdownTimer _asbp_game_mode (+ (Variables|/Game/Blueprints/VehicleBlueprints/BP_GameMode.BP_GameMode_C|GetCountdownTimer _asbp_game_mode) 5.0))
  (Utilities|FlowControl|DoOnce false
    (:Completed
      (Variables|/Game/Blueprints/VehicleBlueprints/BP_GameMode.BP_GameMode_C|SetCommon_amount _asbp_game_mode (- (Variables|/Game/Blueprints/VehicleBlueprints/BP_GameMode.BP_GameMode_C|GetCommon_amount _asbp_game_mode) 1))
      (Actor|DestroyActor)
      (Audio|PlaySound2D "/Game/Sound/Events/pickup.pickup"))))

(fn ConstructionScript)
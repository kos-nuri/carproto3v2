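; Game mode for a kart race whose BeginPlay, Tick and begincountdown events are currently empty, with all logic left in disconnected chains that never run.
; That unused logic shows a paused main menu, locks player input through a looping Delay start countdown, then enables input.
; Another unused chain runs a race timer that destroys the kart and shows the game-over widget at zero.
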(event Custom|begin%20countdown)

(event EventBeginPlay)

(event EventTick
  (params (DeltaSeconds :type Float%20%28single-precision%29))
  ;[1 1 1] Starts to countdown when game starts
)

(fn ConstructionScript)
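; Crash collision component that sends the player back to a checkpoint when a kart hits its owning actor too fast.
; On BeginPlay it unhides the owner's primitive component and binds to its hit event.
; A hit from a BP_KartPawnPlayer at or above a horizontal speed threshold teleports player pawn 0 to that kart's saved checkpoint transform.
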(event Custom|on%20component%20Hit
  (params (HitComponent :type Primitive%20Component%20Object%20Reference) (OtherActor :type Actor%20Object%20Reference) (OtherComp :type Primitive%20Component%20Object%20Reference) (NormalImpulse :type Vector) (Hit :type Hit%20Result%20Structure%20%28by%20ref%29))
  (bind _asbp_kart_pawn_player (Utilities|Casting|CastToBP_KartPawnPlayer OtherActor))
  (if (>= (Variables|/Game/Blueprints/VehicleBlueprints/BP_KartPawnBase.BP_KartPawnBase_C|GetCurrent%20Horizontal%20Speed _asbp_kart_pawn_player) 1.2e+02)
    (Transformation|Teleport (Game|Player|GetPlayerPawn 0) (.location (Variables|/Game/Blueprints/VehicleBlueprints/BP_KartPawnPlayer.BP_KartPawnPlayer_C|GetCheckpoint%20Transform _asbp_kart_pawn_player)) (.rotation (Variables|/Game/Blueprints/VehicleBlueprints/BP_KartPawnPlayer.BP_KartPawnPlayer_C|GetCheckpoint%20Transform _asbp_kart_pawn_player)))))

(event EventBeginPlay
  (bind _returnvalue (Components|GetOwner))
  (bind _returnvalue_2 (Actor|GetComponentbyClass _returnvalue "/Script/Engine.PrimitiveComponent"))
  (Utilities|IsValid _returnvalue_2
    (:Is%20Valid
      (Development|SetHiddeninGame _returnvalue_2 false false)
      (Collision|BindEventtoOnComponentHit _returnvalue_2 (delegate Custom|on%20component%20Hit)))))

(event EventTick
  (params (DeltaSeconds :type Float%20%28single-precision%29)))
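; Player-driven vehicle Blueprint for Konstantine's kart/ship, layering input, respawn setup and HUD on its parent class.
; BeginPlay stores the starting transform as the checkpoint, caches the camera transform and adds a minimap widget.
; Axis inputs feed throttle, steering and a turn-animation value; keys set turn and brake flags, restart the player or quit.
; Speed-based camera zoom and ship tilt logic exist but are disconnected.
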(event EventBeginPlay
  ;[1 1 1] sets initial respawn
  (|CallParentFunction)
  (Utilities|SetInitialRespawn)
  (Utilities|SetCameraTransform)
  (bind _returnvalue (UserInterface|CreateWidget "/Game/Blueprints/VehicleBlueprints/minimap_bp.minimap_bp_C" (Game|GetPlayerController 0)))
  (bind _output_get (Variables|Default|Setminimap_widget _returnvalue))
  (UserInterface|Viewport|AddtoViewport _output_get 0))

(event Collision|EventActorBeginOverlap
  (params (OtherActor :type Actor%20Object%20Reference)))

(event EventTick
  (params (DeltaSeconds :type Float%20%28single-precision%29))
  (|CallParentFunction DeltaSeconds))

(event EventDestroyed)

(event Input|AxisEvents|InputAxisMoveForward
  (params (AxisValue :type Float%20%28single-precision%29))
  (CallFunction|SetThrottleInput AxisValue))

(event Input|AxisEvents|InputAxisMoveRight
  (params (AxisValue :type Float%20%28single-precision%29))
  ;[1 1 1] For turn animation
  (Variables|Default|SetShipTurn (* AxisValue 1e+02)))

(event Input|AxisEvents|InputAxisMoveRight
  (params (AxisValue :type Float%20%28single-precision%29))
  (CallFunction|SetSteeringInput AxisValue))

(event Input|KeyboardEvents|E
  (params (Key :type Key%20Structure))
  (:Pressed
    (Class|GameModeBase|RestartPlayer (Game|GetGameMode))))

(event Input|KeyboardEvents|F10
  (params (Key :type Key%20Structure))
  (:Pressed
    (Game|QuitGame (Game|GetPlayerController 0) "Quit")))

(event Input|KeyboardEvents|S
  (params (Key :type Key%20Structure))
  (:Pressed
    (Variables|Default|SetBraking true))
  (:Released
    (Variables|Default|SetBraking false)))

(event Input|KeyboardEvents|A
  (params (Key :type Key%20Structure))
  (:Pressed
    (Variables|Default|SetTurnLeft true))
  (:Released
    (Variables|Default|SetTurnLeft false)))

(event Input|KeyboardEvents|D
  (params (Key :type Key%20Structure))
  (:Pressed
    (Variables|Default|SetTurnRight true))
  (:Released
    (Variables|Default|SetTurnRight false)))

(fn ConstructionScript
  (|CallParentFunction))
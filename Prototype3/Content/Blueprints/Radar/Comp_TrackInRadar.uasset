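; Actor component that registers its owning actor on the player's HUD radar as either a ground enemy or a pickup.
; BeginPlay calls the add event, which switches on RadarCategory and passes the owner to the matching FlyingGameHUD function of player controller 0.
; A mirrored remove event unregisters the owner by category, but nothing in this graph triggers it.
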(event Custom|EventAddToRadar
  (switch Utilities|FlowControl|Switch|SwitchonEnum_RadarCategories (Variables|Setup|GetRadarCategory)
    (:NewEnumerator1
      ;[1 1 1] Add Ground Enemy
      (bind _asflying_game_hud (Utilities|Casting|CastToFlyingGameHUD (HUD|GetHUD (Game|GetPlayerController 0))))
      (Default|FnAddtoRadarGroundEnemy _asflying_game_hud (Components|GetOwner)))
    (:NewEnumerator3
      ;[1 1 1] Add PickUp
      (bind _asflying_game_hud_2 (Utilities|Casting|CastToFlyingGameHUD (HUD|GetHUD (Game|GetPlayerController 0))))
      (Default|FnAddtoRadarPickUp _asflying_game_hud_2 (Components|GetOwner)))))

(event Custom|EventRemoveFromRadar
  (switch Utilities|FlowControl|Switch|SwitchonEnum_RadarCategories (Variables|Setup|GetRadarCategory)
    (:NewEnumerator1
      ;[1 1 1] Add Ground Enemy
      (bind _asflying_game_hud (Utilities|Casting|CastToFlyingGameHUD (HUD|GetHUD (Game|GetPlayerController 0))))
      (Default|FnRemovefromRadarGroundEnemy _asflying_game_hud (Components|GetOwner)))
    (:NewEnumerator3
      ;[1 1 1] Add PickUp
      (bind _asflying_game_hud_2 (Utilities|Casting|CastToFlyingGameHUD (HUD|GetHUD (Game|GetPlayerController 0))))
      (Default|FnRemovefromRadarPickUp _asflying_game_hud_2 (Components|GetOwner)))))

(event EventBeginPlay
  (CallFunction|EventAddtoRadar))
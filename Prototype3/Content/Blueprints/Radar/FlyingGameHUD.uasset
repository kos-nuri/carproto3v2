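; HUD Blueprint for a flying game that draws a square minimap radar with the player, ground enemies and pickups.
; Actors are added to and removed from the enemy and pickup arrays through its functions.
; Each DrawHUD rescales the radar for the screen resolution, then plots listed actors within horizontal range.
; Dot positions come from inverse-transforming actor locations into player space, so the map rotates with the player, clamped to the radar edges.
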(event EventBeginPlay
  (Variables|Default|SetPlayerRef (Game|Player|GetPlayerPawn 0)))

(event EventDrawHUD
  (params (SizeX :type Integer) (SizeY :type Integer))
  (bind (_x _y) (Radar|FnGetRadarCenterPosition))
  (bind (_x_2 _y_2) (Radar|FnGetRadarCenterPosition))
  (bind (_x_3 _y_3) (Radar|FnGetRadarCenterPosition))
  (bind (_x_4 _y_4) (Radar|FnGetRadarCenterPosition))
  (bind _radarsize (Variables|Radar|GetRadarSize))
  (bind _radarsize_2 (Variables|Radar|GetRadarSize))
  (bind _radarsize_3 (Variables|Radar|GetRadarSize))
  (bind _radarsize_4 (Variables|Radar|GetRadarSize))
  (bind _radarsize_5 (Variables|Radar|GetRadarSize))
  (bind _returnvalue (* _radarsize_4 -1.0))
  (bind _returnvalue_2 (* _radarsize -1.0))
  (if (Variables|Radar|GetShowRadar?)
    (Variables|Radar|SetScreenSize (Math|Vector2D|MakeVector2D (Math|Conversions|ToFloat(Integer) SizeX) (Math|Conversions|ToFloat(Integer) SizeY)))
    (CallFunction|FnScaleRadar SizeX SizeY)
    ;[1 1 1] Draw Radar Background
    (Class|HUD|DrawTextureSimple "/Game/Blueprints/Radar/Textures/Radar_Square.Radar_Square" (- _x_2 _radarsize_3) (- _y_2 _radarsize_3) (Variables|Radar|GetBackgroundScale) false)
    ;[1 1 1] Draw Player
    (Class|HUD|DrawTextureSimple "/Game/Blueprints/Radar/Textures/Minimap_Player_Color.Minimap_Player_Color" _x_4 _y_4 (Variables|Radar|GetPlayerScale) false)
    (Utilities|FlowControl|Sequence
      (:then_1
        ;[1 1 1] Get Ground Enemies
        (for _array_element (Variables|Radar|GetGroundEnemies)
          ;;[1 1 1] Check Range of enemy
          (if (<= (Transformation|GetHorizontalDistanceTo _array_element (Variables|Default|GetPlayerRef)) (Variables|Radar|GetRadarRange))
            ;;[1 1 1] Draw Enemies
            (Class|HUD|DrawTextureSimple "/Game/Blueprints/Radar/Textures/Minimap_GroundEnemy_Color.Minimap_GroundEnemy_Color" (+ (Math|Float|Clamp(Float) (.Y (Radar|FnGetRadarDotPosition _array_element)) _returnvalue _radarsize_5) _x) (+ (Math|Float|Clamp(Float) (* (.X (Radar|FnGetRadarDotPosition _array_element)) -1.0) _returnvalue _radarsize_5) _y) (Variables|Default|GetGroundEnemyScale) false))))
      (:then_3
        ;[1 1 1] Get PickUps
        (for _array_element_2 (Variables|Radar|GetPickUps)
          ;;[1 1 1] Check Range of enemy
          (if (<= (Transformation|GetHorizontalDistanceTo _array_element_2 (Variables|Default|GetPlayerRef)) (Variables|Radar|GetRadarRange))
            ;;[1 1 1] Draw Pick Up
            (Class|HUD|DrawTextureSimple "/Game/Blueprints/Radar/Textures/Minimap_PickUp.Minimap_PickUp" (+ (Math|Float|Clamp(Float) (.Y (Radar|FnGetRadarDotPosition _array_element_2)) _returnvalue_2 _radarsize_2) _x_3) (+ (Math|Float|Clamp(Float) (* (.X (Radar|FnGetRadarDotPosition _array_element_2)) -1.0) _returnvalue_2 _radarsize_2) _y_3) (Variables|Default|GetPickUpScale) false)))))))

(fn ConstructionScript)

(fn FnGetRadarCenterPosition
  (bind _screensize (Variables|Radar|GetScreenSize))
  (bind _radarstartlocation (Variables|Radar|GetRadarStartLocation))
  (bind (_x _y) (Math|Vector2D|BreakVector2D _screensize))
  (bind (_x_2 _y_2) (Math|Vector2D|BreakVector2D _radarstartlocation))
  (return (* _x _x_2) (* _y _y_2)))

(fn FnGetRadarDotPosition
  (params (Actor :type Actor%20Object%20Reference))
  (bind _returnvalue (Transformation|GetActorLocation Actor))
  (bind _playerref (Variables|Default|GetPlayerRef))
  (bind _objectdistancescale (Variables|Radar|GetObjectDistanceScale))
  (bind _returnvalue_2 (Transformation|GetActorTransform _playerref))
  (bind _returnvalue_3 (Math|Transform|InverseTransformLocation _returnvalue_2 _returnvalue))
  (bind _returnvalue_4 (/ _returnvalue_3 _objectdistancescale))
  (bind _returnvalue_5 (Math|Conversions|ToVector2D(Vector) _returnvalue_4))
  (bind (_x _y) (Math|Vector2D|BreakVector2D _returnvalue_5))
  (return _x _y))

(fn FnAddtoRadarGroundEnemy
  (params (Actor :type Actor%20Object%20Reference))
  (Utilities|Array|Add (Variables|Radar|GetGroundEnemies) Actor))

(fn FnRemovefromRadarGroundEnemy
  (params (Actor :type Actor%20Object%20Reference))
  (Utilities|Array|RemoveItem (Variables|Radar|GetGroundEnemies) Actor))

(fn FnScaleRadar
  (params (X :type Integer) (Y :type Integer))
  (if (or (>= X 1920) (>= Y 1040))
    ;[1 1 1] Scale up
    (Variables|Radar|SetRadarSize 2e+02)
    (Variables|Default|SetGroundEnemyScale 0.1)
    (Variables|Default|SetPickUpScale 0.1)
    (Variables|Radar|SetBackgroundScale 1.08)
    (Variables|Radar|SetPlayerScale 0.1)
    (Variables|Radar|SetRadarStartLocation "(X=0.850000,Y=0.750000)")
    (else
      ;[1 1 1] ORIGINAL SIZES
      (Variables|Radar|SetRadarSize 1e+02)
      (Variables|Default|SetGroundEnemyScale 0.05)
      (Variables|Default|SetPickUpScale 0.05)
      (Variables|Radar|SetBackgroundScale 0.54)
      (Variables|Radar|SetPlayerScale 0.05)
      (Variables|Radar|SetRadarStartLocation "(X=0.850000,Y=0.750000)"))))

(fn FnAddtoRadarPickUp
  (params (Actor :type Actor%20Object%20Reference))
  (Utilities|Array|Add (Variables|Radar|GetPickUps) Actor))

(fn FnRemovefromRadarPickUp
  (params (Actor :type Actor%20Object%20Reference))
  (Utilities|Array|RemoveItem (Variables|Radar|GetPickUps) Actor))
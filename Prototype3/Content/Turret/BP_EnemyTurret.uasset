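; Enemy turret that turns to face a TitanfallController pawn spotted by its PawnSensing component and fires on it.
; Each sighting snaps the actor's rotation to the target and, if the fire gate is open, spawns a FirstPersonProjectile pushed along the mesh's forward vector, with sound and looping shoot animation.
; A boolean and Delay throttle the fire rate.
; Tick destroys the turret when Health equals zero; nothing here changes Health.
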(event OnSeePawn(PawnSensing)
  (params (Pawn :type Pawn%20Object%20Reference))
  (bind _returnvalue (Transformation|GetActorLocation))
  (bind _astitanfall_controller (Utilities|Casting|CastToTitanfallController Pawn))
  (Utilities|FlowControl|Sequence
    (:then_0
      (Transformation|SetActorRotation (Math|Rotator|FindLookatRotation _returnvalue (Transformation|GetActorLocation _astitanfall_controller))))
    (:then_1
      (if (Variables|Default|GetSpawnProjectile)
        (bind _returnvalue_2 (Game|SpawnActorfromClass "/Game/FirstPersonBP/Blueprints/FirstPersonProjectile.FirstPersonProjectile_C" (Transformation|GetWorldTransform (Variables|Default|GetProjectileSpawnLocation)) "Undefined" 0 0))
        (Physics|AddImpulse (Variables|/Game/FirstPersonBP/Blueprints/FirstPersonProjectile.FirstPersonProjectile_C|GetSphere _returnvalue_2) (* (Math|Vector|GetForwardVector (Variables|Default|GetSkeletalMesh)) 2.0) "None" false)
        (Audio|PlaySoundatLocation "/Game/StarterContent/Audio/Explosion_Cue.Explosion_Cue" _returnvalue)
        (Components|Animation|PlayAnimation (Variables|Default|GetSkeletalMesh) "/Game/Turret/turret_shoot.turret_shoot" true)
        (Variables|Default|SetSpawnProjectile false)
        (Utilities|FlowControl|Delay 0.5)
        (Variables|Default|SetSpawnProjectile true)))))

(event EventTick
  (params (DeltaSeconds :type Float%20%28single-precision%29))
  (if (== (Variables|Default|GetHealth%20) 0.0)
    (Actor|DestroyActor)))

(fn ConstructionScript)
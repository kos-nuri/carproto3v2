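; BP_HoverVehicle is a player-driven hovercar that moves through physics forces on its CarMesh.
; On BeginPlay it passes CarMesh to four hover components, whose own logic lives outside this Blueprint.
; MoveForward input adds force along the mesh's forward vector, and MoveRight adds yaw torque.
; The steering torque flips sign when velocity along the forward vector is not positive, so turning reverses while backing up.
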(event EventBeginPlay
  (bind _carmesh (Variables|Default|GetCarMesh))
  (Default|InitComponent (Variables|Default|GetBP_HoverComp1) _carmesh)
  (Default|InitComponent (Variables|Default|GetBP_HoverComp2) _carmesh)
  (Default|InitComponent (Variables|Default|GetBP_HoverComp3) _carmesh)
  (Default|InitComponent (Variables|Default|GetBP_HoverComp4) _carmesh))

(event EventTick
  (params (DeltaSeconds :type Float%20%28single-precision%29)))

(event Input|AxisEvents|InputAxisMoveForward
  (params (AxisValue :type Float%20%28single-precision%29))
  (Physics|AddForce (Variables|Default|GetCarMesh) (* (* (Math|Vector|GetForwardVector (Variables|Default|GetCarMesh)) 5e+05) AxisValue) "None" false))

(event Input|AxisEvents|InputAxisMoveRight
  (params (AxisValue :type Float%20%28single-precision%29))
  (bind _returnvalue (Physics|GetPhysicsLinearVelocity (Variables|Default|GetCarMesh) "None"))
  (Class|PrimitiveComponent|AddTorqueinDegrees (Variables|Default|GetCarMesh) (Math|Vector|MakeVector 0.0 0.0 (* (Math|Float|SelectFloat 1.0 -1.0 (> (Math|Vector|DotProduct _returnvalue (Math|Vector|GetForwardVector (Variables|Default|GetCarMesh))) 0.0)) (* AxisValue 3e+08))) "None" false))

(fn ConstructionScript)
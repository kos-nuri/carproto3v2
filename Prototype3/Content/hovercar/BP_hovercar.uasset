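; BP_hovercar is a keyboard-driven physics vehicle that moves and turns by pushing its Cube component.
; W and S set a forward or reverse force, A and D set a yaw torque, and releasing a key zeroes that value.
; Tick applies both to the Cube along the actor's forward and up vectors, without delta-time scaling.
; The graphs contain no hover logic.
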(event EventTick
  (params (DeltaSeconds :type Float%20%28single-precision%29))
  (Physics|AddForce (Variables|Default|GetCube) (* (Transformation|GetActorForwardVector) (Variables|Default|GetForwardForce)) "None" false)
  (Class|PrimitiveComponent|AddTorqueinDegrees (Variables|Default|GetCube) (* (Transformation|GetActorUpVector) (Variables|Default|GetTurnTorque)) "None" false))

(event Input|KeyboardEvents|W
  (params (Key :type Key%20Structure))
  (:Pressed
    (Variables|Default|SetForwardForce 5e+04))
  (:Released
    (Variables|Default|SetForwardForce 0.0)))

(event Input|KeyboardEvents|S
  (params (Key :type Key%20Structure))
  (:Pressed
    (Variables|Default|SetForwardForce -5e+04))
  (:Released
    (Variables|Default|SetForwardForce 0.0)))

(event Input|KeyboardEvents|D
  (params (Key :type Key%20Structure))
  (:Pressed
    (Variables|Default|SetTurnTorque 1e+07))
  (:Released
    (Variables|Default|SetTurnTorque 0.0)))

(event Input|KeyboardEvents|A
  (params (Key :type Key%20Structure))
  (:Pressed
    (Variables|Default|SetTurnTorque -1e+07))
  (:Released
    (Variables|Default|SetTurnTorque 0.0)))

(fn ConstructionScript)
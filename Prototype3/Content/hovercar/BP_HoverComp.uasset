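; BP_HoverComp is a hover thruster component that pushes a physics body away from the surface beneath it.
; InitComponent stores the passed primitive as the parent and enables physics simulation on it.
; Each tick it traces along its negative up vector and, on a hit, applies force along the impact normal at its own location, fading linearly with distance.
; Hits also set high linear and angular damping, which is never reset here.
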(event Custom|InitComponent
  (params (MeshComponent :type Static%20Mesh%20Component%20Object%20Reference))
  (bind _asprimitive_component (Utilities|Casting|CastToPrimitiveComponent MeshComponent))
  (bind _output_get (Variables|Default|SetParentComponent _asprimitive_component))
  (Physics|SetSimulatePhysics _output_get true))

(event EventTick
  (params (DeltaSeconds :type Float%20%28single-precision%29))
  (bind _returnvalue (Transformation|GetWorldLocation))
  (bind _parentcomponent (Variables|Default|GetParentComponent))
  (bind (_outhit _returnvalue_2) (Collision|LineTraceByChannel _returnvalue (+ _returnvalue (* (Math|Vector|GetUpVector) (* (Variables|Default|GetTraceLength) -1.0))) "TraceTypeQuery1" false 0 "ForOneFrame"))
  (if _returnvalue_2
    (Class|PrimitiveComponent|AddForceatLocation (Variables|Default|GetParentComponent) (* (.ImpactNormal (Collision|BreakHitResult _outhit)) (Math|Float|Lerp (Variables|Default|GetHoverForce) 0.0 (/ (Math|Vector|VectorLength (- (.Location (Collision|BreakHitResult _outhit)) (Transformation|GetWorldLocation))) (Variables|Default|GetTraceLength)))) (Transformation|GetWorldLocation) "None")
    (Class|PrimitiveComponent|SetLinearDamping _parentcomponent 1e+01)
    (Class|PrimitiveComponent|SetAngularDamping _parentcomponent 15.0)))
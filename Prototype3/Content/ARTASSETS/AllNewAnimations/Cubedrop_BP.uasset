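; Actor Blueprint, named as a cube drop, that animates its static mesh vertically in world space from BeginPlay.
; Timeline_0 adds its track value to the mesh's current Z on each update, feeding a five-second Delay that starts Timeline_1.
; Timeline_1 adds its track to HeadWorldLocZ, which Tick refreshes from the mesh's current Z, so both offsets accumulate rather than being relative to a fixed start.
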(event EventBeginPlay
  (bind _staticmeshcomponent0 (Variables|Default|GetStaticMeshComponent0))
  (bind _staticmeshcomponent0_2 (Variables|Default|GetStaticMeshComponent0))
  (bind _returnvalue (Transformation|GetWorldLocation _staticmeshcomponent0))
  (bind _returnvalue_2 (Transformation|GetWorldLocation _staticmeshcomponent0_2))
  (bind _newtrack_0 (Timeline|Timeline_0 Play)
    (:Update
      (Transformation|SetWorldLocation (Variables|Default|GetStaticMeshComponent0) (Math|Vector|MakeVector (.x _returnvalue_2) (.y _returnvalue_2) (+ (.z _returnvalue_2) _newtrack_0)) false false)
      (Utilities|FlowControl|Delay 5.0)
      (bind _newtrack_0_2 (Timeline|Timeline_1 Play)
        (:Update
          (Transformation|SetWorldLocation (Variables|Default|GetStaticMeshComponent0) (Math|Vector|MakeVector (.x _returnvalue) (.y _returnvalue) (+ (Variables|Default|GetHeadWorldLocZ) _newtrack_0_2)) false false))))))

(event Collision|EventActorBeginOverlap
  (params (OtherActor :type Actor%20Object%20Reference)))

(event EventTick
  (params (DeltaSeconds :type Float%20%28single-precision%29))
  (Variables|Default|SetHeadWorldLocZ (.z (Transformation|GetWorldLocation (Variables|Default|GetStaticMeshComponent0)))))

(fn ConstructionScript)
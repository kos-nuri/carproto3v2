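; BP_SPEEEED is a boost trigger among the spline track assets that speeds up any VehicleBlueprint overlapping its box.
; On overlap it attaches a rotated dash particle effect to the vehicle's Hovership component.
; It adds 1.25 times the current physics velocity on top of the existing one, so the vehicle leaves at 2.25 times its speed.
; After a half-second delay the effect is deactivated, while the velocity is left as is.
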(event OnComponentBeginOverlap(Box)
  (params (OverlappedComponent :type Primitive%20Component%20Object%20Reference) (OtherActor :type Actor%20Object%20Reference) (OtherComp :type Primitive%20Component%20Object%20Reference) (OtherBodyIndex :type Integer) (bFromSweep :type Boolean) (SweepResult :type Hit%20Result%20Structure%20%28by%20ref%29))
  (bind _asvehicle_blueprint (Utilities|Casting|CastToVehicleBlueprint OtherActor))
  (bind _returnvalue (Effects|SpawnEmitterAttached "/Game/VFX/Particles/p_dash.p_dash" (Variables|/Game/BP_CODE/VehicleAdvBP/Blueprints/VehicleBlueprint.VehicleBlueprint_C|Gethovership _asvehicle_blueprint) "None" "0, 0, 0" "0,90.000000, 0"))
  (bind _returnvalue_2 (Physics|GetPhysicsLinearVelocity (Variables|/Script/Engine.MovementComponent|GetUpdatedPrimitive (Variables|/Script/PhysXVehicles.WheeledVehicle|GetVehicleMovement _asvehicle_blueprint)) "None"))
  (Physics|SetPhysicsLinearVelocity (Variables|/Script/Engine.MovementComponent|GetUpdatedPrimitive (Variables|/Script/PhysXVehicles.WheeledVehicle|GetVehicleMovement _asvehicle_blueprint)) (* _returnvalue_2 1.25) true "None")
  (Utilities|FlowControl|Delay 0.5)
  (Components|Activation|Deactivate _returnvalue))

(event EventBeginPlay)

(event Collision|EventActorBeginOverlap
  (params (OtherActor :type Actor%20Object%20Reference)))

(event EventTick
  (params (DeltaSeconds :type Float%20%28single-precision%29)))

(fn ConstructionScript)